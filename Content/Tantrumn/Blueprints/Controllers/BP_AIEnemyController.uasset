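; AI controller for enemies that runs the BP_AIEnemyBT behavior tree on BeginPlay and feeds it perception results through the blackboard.
; A perceived throwable sets CanSeeThrowable and the Throwable object, but only while HasThrowable is false; a perceived player sets CanSeePlayer and Player.
; Neither flag is cleared here, since the stimulus's sensed state is not checked.
; Each perception update also draws short-lived debug lines from the pawn to the updated actors.
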(event `self.ReceiveBeginPlay`
  (`self.RunBehaviorTree` "/Game/Tantrumn/Blueprints/Controllers/BP_AIEnemyBT.BP_AIEnemyBT"))

(event `self.AIPerception.OnTargetPerceptionUpdated`
  (params (Actor :type "Actor Object Reference") (Stimulus :type "AIStimulus Structure"))
  (bind _returnvalue (`AIBlueprintHelperLibrary.GetBlackboard` null))
  (bind _returnvalue_2 (`AIBlueprintHelperLibrary.GetBlackboard` null))
  (cast `/Game/Tantrumn/Blueprints/Characters/BP_ThrowableActor` Actor
    (:`then`
      (if (not (`BlackboardComponent.GetValueAsBool` (`AIBlueprintHelperLibrary.GetBlackboard` null) "HasThrowable"))
        ;[1 1 1] If throwable seen, make CanSeeThrowable true
        (`BlackboardComponent.SetValueAsBool` _returnvalue_2 "CanSeeThrowable" true)
        (`BlackboardComponent.SetValueAsObject` _returnvalue_2 "Throwable" Actor)))
    (:`CastFailed`
      (cast `/Game/Tantrumn/Blueprints/Characters/BP_Player` Actor)
      ;[1 1 1] If player seen, make CanSeePlayer true
      (`BlackboardComponent.SetValueAsBool` _returnvalue "CanSeePlayer" true)
      (`BlackboardComponent.SetValueAsObject` _returnvalue "Player" Actor))))

(event `self.AIPerception.OnPerceptionUpdated`
  (params (UpdatedActors :type "Array of Actor Object Reference (by ref)"))
  (for _array_element UpdatedActors
    (`KismetSystemLibrary.DrawDebugLine` (`self.K2_GetActorLocation` (`self.K2_GetPawn`)) (`self.K2_GetActorLocation` _array_element) (struct :`R` 0.921875 :`B` 0.016411 :`A` 1.0) 0.5 2.0)))

(fn `UserConstructionScript`)