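; Behavior tree task that makes a BP_AIEnemy pick up a throwable by requesting a pull.
; It writes ThrowableActor to the Throwable blackboard key; for a BP_ThrowableActor, it calls PickedUpDeReg and turns the enemy toward it using only X and Z coordinates.
; It then calls RequestPullObject, sets HasThrowable and finishes successfully without waiting on the pull.
; A failed pawn cast never finishes the task.
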(event `self.ReceiveExecuteAI`
  (params (OwnerController :type "AIController Object Reference") (ControlledPawn :type "Pawn Object Reference"))
  (bind (_returnvalue_x _returnvalue_y _returnvalue_z) (`KismetMathLibrary.BreakVector` (`Actor.K2_GetActorLocation` ControlledPawn)))
  (bind (_returnvalue_x_2 _returnvalue_y_2 _returnvalue_z_2) (`KismetMathLibrary.BreakVector` (`Actor.K2_GetActorLocation` (`BTFunctionLibrary.GetBlackboardValueAsActor` (`self.Throwable`)))))
  (`BTFunctionLibrary.SetBlackboardValueAsObject` (`self.Throwable`) (`self.ThrowableActor`))
  (bind _asbp_aienemy (cast `/Game/Tantrumn/Blueprints/Characters/BP_AIEnemy` ControlledPawn))
  (bind _asbp_throwable_actor (cast `/Game/Tantrumn/Blueprints/Characters/BP_ThrowableActor` (`self.ThrowableActor`))
    (:`then`
      (`/Game/Tantrumn/Blueprints/Characters/BP_ThrowableActor.PickedUpDeReg` _asbp_throwable_actor)
      (`Actor.K2_SetActorRotation` _asbp_aienemy (`KismetMathLibrary.FindLookAtRotation` (`KismetMathLibrary.MakeVector` _returnvalue_x 0.0 _returnvalue_z) (`KismetMathLibrary.MakeVector` _returnvalue_x_2 0.0 _returnvalue_z_2)) false))
    (:`CastFailed`
      _))
  (`TantrumnCharacterBase.RequestPullObject` _asbp_aienemy)
  (`BTFunctionLibrary.SetBlackboardValueAsBool` (`self.HasThrowable`) true)
  (`self.FinishExecute` true))