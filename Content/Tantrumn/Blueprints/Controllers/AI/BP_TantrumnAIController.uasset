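; AI controller for Tantrumn that runs a race or battle behavior tree depending on the active game mode.
; On BeginPlay it writes the first level-end trigger (race) or first throwable actor (battle) location into the Blackboard.
; Tick mirrors the game state's IsPlaying flag to the Blackboard.
; AI perception records player visibility and the player reference there, and draws debug lines to perceived players.
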(event `self.ReceiveBeginPlay`
  (bind _returnvalue (`GameplayStatics.GetGameMode`))
  (cast `/Game/Tantrumn/Blueprints/GameModes/BP_TantrumnGameModeBaseRace` _returnvalue
    (:`then`
      (`self.RunBehaviorTree` "/Game/Tantrumn/Blueprints/Controllers/AI/BT_AIRace.BT_AIRace")
      (`self.SetRaceEndAsDestination`))
    (:`CastFailed`
      (cast `/Game/Tantrumn/Blueprints/GameModes/BP_TantrumnGameModeBaseBattle` _returnvalue)
      (`self.RunBehaviorTree` "/Game/Tantrumn/Blueprints/Controllers/AI/BT_AIBattle.BT_AIBattle")
      (`self.SetThrowableAsPosition`))))

(event `self.ReceiveTick`
  (params (DeltaSeconds :type "Float (single-precision)"))
  ;[1 1 1] Set IsPlaying
  (bind _astantrumn_game_state_base (cast `TantrumnGameStateBase` (`GameplayStatics.GetGameState`)))
  (`BlackboardComponent.SetValueAsBool` (`self.Blackboard`) "IsPlaying" (`TantrumnGameStateBase.IsPlaying` _astantrumn_game_state_base)))

(event `self.AIPerception.OnTargetPerceptionUpdated`
  (params (Actor :type "Actor Object Reference") (Stimulus :type "AIStimulus Structure"))
  (bind _blackboard (`self.Blackboard`))
  ;[1 1 1] Perception Conditions
  (if (== (`GameplayStatics.GetObjectClass` Actor) "/Game/Tantrumn/Blueprints/Characters/BP_Player.BP_Player_C")
    (`BlackboardComponent.SetValueAsBool` _blackboard "CanSeePlayer" (`.bSuccessfullySensed` (break `AIStimulus` Stimulus)))
    (`BlackboardComponent.SetValueAsObject` _blackboard "Player" Actor)))

(event `self.AIPerception.OnPerceptionUpdated`
  (params (UpdatedActors :type "Array of Actor Object Reference (by ref)"))
  ;[1 1 1] Perception Check
  (`/Engine/EditorBlueprintResources/StandardMacros.IsValid` null
    (:`Is Valid`
      (for _array_element UpdatedActors
        (cast `/Game/Tantrumn/Blueprints/Characters/BP_Player` _array_element)
        (`KismetSystemLibrary.DrawDebugLine` (`self.K2_GetActorLocation` (`self.K2_GetPawn`)) (`self.K2_GetActorLocation` _array_element) (struct :`R` 0.921875 :`B` 0.016411 :`A` 1.0) 0.5 2.0)))))

(fn `SetRaceEndAsDestination`
  (bind _outactors (`GameplayStatics.GetAllActorsOfClass` "/Script/Tantrumn.TantrumnLevelEndTrigger"))
  (if (> (`KismetArrayLibrary.Array_Length` _outactors) 0)
    (`BlackboardComponent.SetValueAsVector` (`self.Blackboard`) "Destination" (`self.K2_GetActorLocation` (`|GetArrayItem` _outactors)))))

(fn `SetThrowableAsPosition`
  (bind _outactors (`GameplayStatics.GetAllActorsOfClass` "/Game/Tantrumn/Blueprints/AIActors/BP_ThrowableActor.BP_ThrowableActor_C"))
  (if (> (`KismetArrayLibrary.Array_Length` _outactors) 0)
    (`BlackboardComponent.SetValueAsVector` (`self.Blackboard`) "ThrowablePosition" (`self.K2_GetActorLocation` (`|GetArrayItem` _outactors)))))

(fn `UserConstructionScript`)