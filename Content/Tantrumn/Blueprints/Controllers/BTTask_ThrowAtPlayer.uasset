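; Behavior Tree task that makes a BP_AIEnemy throw its held object at the player.
; It applies a single RInterpTo step toward the look-at rotation of the PlayerPosition blackboard actor, with no delta time supplied, then requests the throw.
; It clears the HasThrowable blackboard flag and finishes successfully right away, without waiting for the throw to complete.
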(event `self.ReceiveExecuteAI`
  (params (OwnerController :type "AIController Object Reference") (ControlledPawn :type "Pawn Object Reference"))
  (bind _asbp_aienemy (cast `/Game/Tantrumn/Blueprints/Characters/BP_AIEnemy` ControlledPawn))
  (`Actor.K2_SetActorRotation` _asbp_aienemy (`KismetMathLibrary.RInterpTo` (`Actor.K2_GetActorRotation` _asbp_aienemy) (`KismetMathLibrary.FindLookAtRotation` (`Actor.K2_GetActorLocation` _asbp_aienemy) (`Actor.K2_GetActorLocation` (`BTFunctionLibrary.GetBlackboardValueAsActor` (`self.PlayerPosition`)))) 0.0 0.5) false)
  (`TantrumnCharacterBase.RequestThrowObject` _asbp_aienemy)
  (`BTFunctionLibrary.SetBlackboardValueAsBool` (`self.HasThrowable`))
  (`self.FinishExecute` true))